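; Test Blueprint that animates the "App" scalar parameter on every material of its skeletal mesh when play begins.
; BeginPlay creates a dynamic material instance per material slot and stores them in an array.
; A timeline then writes its track value to all instances on each update, with debug prints along the way.
; An unconnected single-slot variant of the same logic remains in the graph and never runs.
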(event `self.ReceiveBeginPlay`
  (for (_ _array_index) (`MeshComponent.GetMaterials` (`self.SkeletalMesh`))
    (bind _returnvalue (`PrimitiveComponent.CreateDynamicMaterialInstance` (`self.SkeletalMesh`) _array_index null "None"))
    (`KismetArrayLibrary.Array_Add` (`self.NewVar_0`) _returnvalue)
    (`KismetSystemLibrary.PrintString` (`KismetSystemLibrary.GetDisplayName` _returnvalue)))
  (`KismetSystemLibrary.PrintString` (`KismetStringLibrary.Conv_IntToString` (`KismetArrayLibrary.Array_Length` (`self.NewVar_0`))))
  (bind (_direction _newtrack_0) (`Timeline|Timeline_0` :!via `PlayFromStart`)
    (:`Update`
      (`KismetSystemLibrary.PrintString` (`KismetStringLibrary.Concat_StrStr` "current value " (`KismetStringLibrary.Conv_DoubleToString` _newtrack_0)) true true (struct :`G` 0.66 :`B` 1.0 :`A` 1.0) 0.0)
      (for _array_element (`self.NewVar_0`)
        (`MaterialInstanceDynamic.SetScalarParameterValue` _array_element "App" _newtrack_0)))))

(fn `UserConstructionScript`)