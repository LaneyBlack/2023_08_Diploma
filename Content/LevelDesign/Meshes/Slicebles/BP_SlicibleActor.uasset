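; Sliceable actor that can be cut in two along a plane, with both halves then falling as physics objects.
; At BeginPlay it copies its static mesh into a procedural mesh and destroys the original.
; SliceActor slices that mesh with a capped cut at an offset point and pushes both halves with the same impulse.
; If dissolve is enabled, glowing dynamic materials are animated by a timeline, then the actor destroys itself.
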(event `self.ReceiveBeginPlay`
  (`KismetProceduralMeshLibrary.CopyProceduralMeshFromStaticMeshComponent` (`self.StaticMesh`) 0 (`self.ProceduralMesh`) true)
  (`SceneComponent.K2_SetWorldTransform` (`self.ProceduralMesh`) (`SceneComponent.K2_GetComponentToWorld` (`self.StaticMesh`)) false false)
  (`ActorComponent.K2_DestroyComponent` (`self.StaticMesh`)))

(event `self.SliceActor`
  (params (SliceVector :type "Vector Structure (by ref)") (CollisionPoint :type "Vector Structure (by ref)"))
  (bind _proceduralmesh (`self.ProceduralMesh`))
  (set `self.Alt Collision Point` (+ (`self.Alt Collision Point`) (`self.K2_GetActorLocation`)))
  (set `self.Collision Point` CollisionPoint)
  (set `self.Plane Normal` (* SliceVector (`KismetMathLibrary.SignOfFloat` (`KismetMathLibrary.Dot_VectorVector` SliceVector (0.0 0.0 1.0)))))
  (bind _outotherhalfprocmesh (`KismetProceduralMeshLibrary.SliceProceduralMesh` (`self.ProceduralMesh`) (`self.Alt Collision Point`) (`self.Plane Normal`) true "CreateNewSectionForCap" (`self.Cap Material`)))
  (bind _output_get (set `self.Other Cut Half` _outotherhalfprocmesh))
  (set `self.ImpulseVector` (* (`KismetMathLibrary.Normal` (`KismetMathLibrary.SelectVector` (+ (`self.Plane Normal`) (`self.GetActorForwardVector`)) (`self.GetActorForwardVector`) (`self.Use Plane Normal`))) (`self.ImpactStreangth`)))
  (`PrimitiveComponent.SetSimulatePhysics` _output_get true)
  (`PrimitiveComponent.AddImpulseAtLocation` (`self.Other Cut Half`) (`self.ImpulseVector`) (`self.Alt Collision Point`) "None")
  (`PrimitiveComponent.SetSimulatePhysics` _proceduralmesh true)
  (`PrimitiveComponent.AddImpulseAtLocation` _proceduralmesh (`self.ImpulseVector`) (`self.Alt Collision Point`) "None")
  (if (`self.Should Dissolve`)
    (`|ExecutionSequence`
      (:`then_0`
        (`self.SetMaterials` (`self.ProceduralMesh`))
        (`self.SetMaterials` (`self.Other Cut Half`)))
      (:`then_1`
        (`TimelineComponent.SetPlayRate` (`self.Timeline_0`) (/ 1.0 (`self.Time To Dissolve`)))
        (bind (_direction _newtrack_0) (`Timeline|Timeline_0` :!via `PlayFromStart`)
          (:`Update`
            (for _array_element (`self.DynamicMaterials`)
              (`MaterialInstanceDynamic.SetScalarParameterValue` _array_element "App" _newtrack_0)))
          (:`Finished`
            (`self.K2_DestroyActor`)))))))

(fn `DrawDebugSliceProperties`
  (bind _collision_point (`self.Collision Point`))
  (`KismetSystemLibrary.DrawDebugArrow` _collision_point (+ _collision_point (* (`self.Plane Normal`) 50.0)) 5.0 (struct :`R` 0.855615 :`B` 1.0 :`A` 1.0) 10000.0 2.0)
  (`KismetSystemLibrary.DrawDebugPlane` (`KismetMathLibrary.MakePlaneFromPointAndNormal` (`self.Collision Point`) (`self.Plane Normal`)) (`self.Collision Point`) 100.0 (struct :`G` 0.267682 :`B` 1.0 :`A` 0.5) 1000.0)
  (`KismetSystemLibrary.PrintString` (`KismetStringLibrary.Concat_StrStr` "Hit Location " (`KismetStringLibrary.Conv_VectorToString` (`self.Collision Point`))) true true (struct :`R` 0.082624 :`G` 1.0 :`A` 1.0) 5.0)
  (`KismetSystemLibrary.PrintString` (`KismetStringLibrary.Concat_StrStr` "Plane Normal " (`KismetStringLibrary.Conv_VectorToString` (`self.Plane Normal`))) true true (struct :`R` 0.082624 :`G` 1.0 :`A` 1.0) 5.0))

(fn `Set mats`)

(fn `SetMaterials`
  (params (Target :type "MeshComponent Object Reference"))
  (for (_ _array_index) (`MeshComponent.GetMaterials` Target)
    (bind _returnvalue (`PrimitiveComponent.CreateDynamicMaterialInstance` Target _array_index null "None"))
    (`KismetArrayLibrary.Array_Add` (`self.DynamicMaterials`) _returnvalue)
    (`MaterialInstanceDynamic.SetVectorParameterValue` _returnvalue "Col" (struct :`R` 1.0 :`G` 0.026228 :`A` 1.0))
    (`MaterialInstanceDynamic.SetScalarParameterValue` _returnvalue "Emm" 10000.0)))

(fn `UserConstructionScript`)