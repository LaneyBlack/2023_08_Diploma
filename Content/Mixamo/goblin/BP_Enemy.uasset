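; BP_Enemy is an enemy Blueprint, filed under the Mixamo goblin assets, that loses health when hit and is destroyed when it runs out.
; The GetHit event calls TakeDamage to subtract a fixed amount of Health, prints the result, then destroys the actor at zero or below.
; An IsGettingHit flag ignores repeat hits until a short retriggerable delay clears it.
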(event `GetHit`
  ;[0.2031 0.2031 0.2031] Get Hit
  (if (not (`self.IsGettingHit`))
    (set `self.IsGettingHit` true)
    (`self.takeDamage `)
    (`KismetSystemLibrary.PrintString` (`KismetStringLibrary.Conv_DoubleToString` (`self.Health`)))
    (if (<= (`self.Health`) 0.0)
      (`self.K2_DestroyActor`)
      (else
        (`KismetSystemLibrary.RetriggerableDelay` 1.0)
        (set `self.IsGettingHit` false)))))

(fn `takeDamage `
  (set `self.Health` (- (`self.Health`) 25.0)))

(fn `UserConstructionScript`)