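; BP_CombatTutorialCheckpoint is a trigger actor that starts a combat tutorial when the player character enters it.
; Its Box overlap checks that the TutorialComponent's Deleyed flag is unset and that the overlapping actor is BP_ThirdPersonCharacter, then calls FireTutorial on that component.
; BeginPlay, Tick, actor overlap and construction only pass through to the parent class.
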(event `self.ReceiveBeginPlay`
  (`parent.ReceiveBeginPlay`))

(event `self.ReceiveActorBeginOverlap`
  (params (OtherActor :type "Actor Object Reference"))
  (`parent.ReceiveActorBeginOverlap` OtherActor))

(event `self.ReceiveTick`
  (params (DeltaSeconds :type "Float (single-precision)"))
  (`parent.ReceiveTick` DeltaSeconds))

(event `self.Box.OnComponentBeginOverlap`
  (params (OverlappedComponent :type "PrimitiveComponent Object Reference") (OtherActor :type "Actor Object Reference") (OtherComp :type "PrimitiveComponent Object Reference") (OtherBodyIndex :type Integer) (bFromSweep :type Boolean) (SweepResult :type "HitResult Structure (by ref)"))
  (if (not (`/Game/Tutorial_Utilities/Components/TutorialComponent.Deleyed` (`self.TutorialComponent`)))
    (cast `/Game/ThirdPerson/Blueprints/BP_ThirdPersonCharacter` OtherActor)
    (`/Game/Tutorial_Utilities/Components/TutorialComponent.FireTutorial` (`self.TutorialComponent`))))

(fn `UserConstructionScript`
  (`parent.UserConstructionScript`))