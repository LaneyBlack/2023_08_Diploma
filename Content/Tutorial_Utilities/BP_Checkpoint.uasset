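; Checkpoint actor that updates the player's respawn point the first time the third-person character overlaps its trigger box.
; The overlap writes a respawn transform to the PlayerGameMode, using the checkpoint's location with the character's rotation and scale.
; It also stores its CurrentWorld value as the respawn level, prints a debug message and latches Triggered so it fires only once.
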(event `self.ReceiveBeginPlay`)

(event `self.Box.OnComponentBeginOverlap`
  (params (OverlappedComponent :type "PrimitiveComponent Object Reference") (OtherActor :type "Actor Object Reference") (OtherComp :type "PrimitiveComponent Object Reference") (OtherBodyIndex :type Integer) (bFromSweep :type Boolean) (SweepResult :type "HitResult Structure (by ref)"))
  (if (not (`self.Triggered`))
    (bind _asbp_third_person_character (cast `/Game/ThirdPerson/Blueprints/BP_ThirdPersonCharacter` OtherActor))
    (bind _asplayer_game_mode (cast `/Game/GameModes/PlayerGameMode` (`GameplayStatics.GetGameMode`)))
    (bind (_returnvalue_location _returnvalue_rotation _returnvalue_scale) (`KismetMathLibrary.BreakTransform` (`self.GetTransform` _asbp_third_person_character)))
    (set `/Game/GameModes/PlayerGameMode.Respawn Transform` (`KismetMathLibrary.MakeTransform` (`self.K2_GetActorLocation`) _returnvalue_rotation _returnvalue_scale) _asplayer_game_mode)
    (bind _asplayer_game_mode_2 (cast `/Game/GameModes/PlayerGameMode` (`GameplayStatics.GetGameMode`)))
    (set `/Game/GameModes/PlayerGameMode.RespawnLevel` (`self.CurrentWorld`) _asplayer_game_mode_2)
    (`KismetSystemLibrary.PrintString` "checkpoint")
    (set `self.Triggered` true)))

(fn `UserConstructionScript`)