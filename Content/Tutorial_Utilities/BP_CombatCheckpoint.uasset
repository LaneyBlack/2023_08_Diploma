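; Combat checkpoint actor that tracks an enemy encounter and moves the player's respawn point once it is cleared.
; Player overlap sets the game mode's respawn level and starts a fast polling timer over enemies overlapping the referenced nav mesh volume.
; When the IsGettingHit count matches the enemy total, it clears that level and sets a sanitized post-combat respawn transform.
; It optionally plays timeline-driven slow motion, then caches combo points after a delay.
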(event `self.ReceiveBeginPlay`
  (`parent.ReceiveBeginPlay`)
  (set `self.PlayerSafeCombatSpawn` (`self.SanitizeSpawnPosition` (`self.PlayerSpawnAfterCombat`) (`self.K2_GetActorLocation`))))

(event `self.Box.OnComponentBeginOverlap`
  (params (OverlappedComponent :type "PrimitiveComponent Object Reference") (OtherActor :type "Actor Object Reference") (OtherComp :type "PrimitiveComponent Object Reference") (OtherBodyIndex :type Integer) (bFromSweep :type Boolean) (SweepResult :type "HitResult Structure (by ref)"))
  (if (not (`self.Triggered`))
    (cast `/Game/ThirdPerson/Blueprints/BP_ThirdPersonCharacter` OtherActor)
    (bind _asplayer_game_mode (cast `/Game/GameModes/PlayerGameMode` (`GameplayStatics.GetGameMode`)))
    (set `/Game/GameModes/PlayerGameMode.RespawnLevel` (`self.CurrentWorld`) _asplayer_game_mode)
    (bind _output_get (set `self.TotalEnemies` (`KismetArrayLibrary.Array_Length` (`self.EnemiesInEncouter`))))
    (if (> _output_get 0)
      (bind _returnvalue (`KismetSystemLibrary.K2_SetTimerDelegate` (delegate `CustomEvent`) 0.025 true))
      (set `self.CombatTimer` _returnvalue))))

(event `CustomEvent`
  (bind _returnvalue (`ComboSystem.GetInstance`))
  (`self.DetermineEnemiesInEncounter`)
  (set `self.DeadCount` 0)
  (for _array_element (`self.EnemiesInEncouter`)
    (bind _asbase_enemy (cast `BaseEnemy` _array_element))
    (if (`BaseEnemy.bIsGettingHit` _asbase_enemy)
      (`/Engine/EditorBlueprintResources/StandardMacros.IncrementInt` (`self.DeadCount`))))
  (if (== (`self.DeadCount`) (`self.TotalEnemies`))
    (`KismetSystemLibrary.K2_ClearAndInvalidateTimerHandle` (`self.CombatTimer`))
    (bind _asplayer_game_mode (cast `/Game/GameModes/PlayerGameMode` (`GameplayStatics.GetGameMode`)))
    (set `/Game/GameModes/PlayerGameMode.RespawnLevel` (struct) _asplayer_game_mode)
    (`KismetSystemLibrary.PrintString` "all killed" true true (struct :`R` 1.0 :`B` 0.079724 :`A` 1.0))
    (bind _asplayer_game_mode_2 (cast `/Game/GameModes/PlayerGameMode` (`GameplayStatics.GetGameMode`)))
    (bind (_respawn_transform_location _respawn_transform_rotation _respawn_transform_scale) (`KismetMathLibrary.BreakTransform` (`/Game/GameModes/PlayerGameMode.Respawn Transform` _asplayer_game_mode_2)))
    (set `/Game/GameModes/PlayerGameMode.Respawn Transform` (`KismetMathLibrary.MakeTransform` (`self.PlayerSafeCombatSpawn`) (`SceneComponent.K2_GetComponentRotation` (`self.AfterEncounter`)) _respawn_transform_scale) _asplayer_game_mode_2)
    (set `self.Active` false)
    (`|ExecutionSequence`
      (:`then_0`
        (if (`self.SlowMoOnLastKill`)
          (bind (_direction _newtrack_0) (`Timeline|Timeline` :!via `PlayFromStart`)
            (:`Update`
              (`GameplayStatics.SetGlobalTimeDilation` (`KismetMathLibrary.Lerp` 1.0 0.05 _newtrack_0))))))
      (:`then_1`
        ;[1 1 1] SUCKS A DICK
        (`KismetSystemLibrary.Delay` 2.1)
        (set `ComboSystem.ComboCache` (`ComboSystem.AbilityComboPoints` _returnvalue) _returnvalue)))))

(fn `DetermineEnemiesInEncounter`
  (bind _output_get (set `self.EnemiesInEncouter` (`self.GetOverlappingActors` (`self.NavMeshReference`) "/Script/TheFallenSamurai.BaseEnemy"))))

(fn `UserConstructionScript`
  (`parent.UserConstructionScript`))