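; BP_ParryCheckpoint is a tutorial trigger that stages a parry lesson against a linked TutorialEnemy.
; When active, overlapping its box freezes the third-person character's movement and uses a timeline to turn the control rotation toward the enemy.
; The enemy's parry event drops global time dilation into heavy slow motion; its successful-parry event restores normal time and walking movement.
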(event `self.ReceiveBeginPlay`
  (bind _tutorialenemy (`self.TutorialEnemy`))
  (`parent.ReceiveBeginPlay`)
  (add `/Game/Enemy/BP_BaseEnemy.ParryEvent` _tutorialenemy (delegate `CustomEvent_0`))
  (add `/Game/Enemy/BP_BaseEnemy.SuccessfulParryEvent` _tutorialenemy (delegate `CustomEvent_1`)))

(event `CustomEvent_0`
  (`GameplayStatics.SetGlobalTimeDilation` 0.05))

(event `CustomEvent_1`
  (bind _character_movement (`self.Character Movement`))
  (`GameplayStatics.SetGlobalTimeDilation` 1.0)
  (`/Engine/EditorBlueprintResources/StandardMacros.IsValid` _character_movement
    (:`Is Valid`
      (`CharacterMovementComponent.SetMovementMode` _character_movement "MOVE_Walking" 0))))

(event `self.ReceiveActorBeginOverlap`
  (params (OtherActor :type "Actor Object Reference"))
  (`parent.ReceiveActorBeginOverlap` OtherActor))

(event `self.ReceiveTick`
  (params (DeltaSeconds :type "Float (single-precision)"))
  (`parent.ReceiveTick` DeltaSeconds))

(event `self.Box.OnComponentBeginOverlap`
  (params (OverlappedComponent :type "PrimitiveComponent Object Reference") (OtherActor :type "Actor Object Reference") (OtherComp :type "PrimitiveComponent Object Reference") (OtherBodyIndex :type Integer) (bFromSweep :type Boolean) (SweepResult :type "HitResult Structure (by ref)"))
  (if (`self.Active`)
    (bind _asbp_third_person_character (cast `/Game/ThirdPerson/Blueprints/BP_ThirdPersonCharacter` OtherActor))
    (set `self.CharacterContorler` (`Pawn.GetController` _asbp_third_person_character))
    (bind _charactermovement (`Character.CharacterMovement` _asbp_third_person_character))
    (set `self.Character Movement` _charactermovement)
    (`MovementComponent.StopMovementImmediately` _charactermovement)
    (set `self.ControlRotation` (`Controller.GetControlRotation` (`self.CharacterContorler`)))
    (set `self.TargetRotation` (`KismetMathLibrary.FindLookAtRotation` (`self.K2_GetActorLocation` _asbp_third_person_character) (`self.K2_GetActorLocation` (`self.TutorialEnemy`))))
    (`CharacterMovementComponent.SetMovementMode` (`self.Character Movement`) "MOVE_None" 0)
    (bind (_direction _alpha) (`Timeline|Timeline_0` :!via `PlayFromStart`)
      (:`Update`
        (`Controller.SetControlRotation` (`self.CharacterContorler`) (`KismetMathLibrary.RLerp` (`self.ControlRotation`) (`self.TargetRotation`) _alpha true))))))

(fn `UserConstructionScript`
  (`parent.UserConstructionScript`))