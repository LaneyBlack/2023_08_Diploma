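; BP_TutorialCheckpoint is a trigger actor that starts a tutorial when the player character enters its box.
; On box overlap it checks that neither its Triggered flag nor the TutorialComponent's delayed flag is set, then filters for BP_ThirdPersonCharacter.
; It hands off to FireTutorial on the TutorialComponent; an older direct add-widget call remains unconnected, and this graph never sets Triggered.
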(event `self.Box.OnComponentBeginOverlap`
  (params (OverlappedComponent :type "PrimitiveComponent Object Reference") (OtherActor :type "Actor Object Reference") (OtherComp :type "PrimitiveComponent Object Reference") (OtherBodyIndex :type Integer) (bFromSweep :type Boolean) (SweepResult :type "HitResult Structure (by ref)"))
  (if (and (not (`self.Triggered`)) (not (`/Game/Tutorial_Utilities/Components/TutorialComponent.Deleyed` (`self.TutorialComponent`))))
    (cast `/Game/ThirdPerson/Blueprints/BP_ThirdPersonCharacter` OtherActor)
    (`/Game/Tutorial_Utilities/Components/TutorialComponent.FireTutorial` (`self.TutorialComponent`))))

(fn `UserConstructionScript`
  (`parent.UserConstructionScript`))