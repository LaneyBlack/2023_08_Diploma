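; Tutorial checkpoint trigger that, on the player's first overlap, saves the respawn transform and level to PlayerGameMode and shows a timed tutorial widget.
; With a valid world asset, it counts BP_BaseEnemy actors and polls by timer while the streamed level is loaded.
; When all enemies report IsGettingHit, it sets the next level and plays a slow-motion timeline whose play rate compensates for global time dilation.
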(event `self.ReceiveBeginPlay`
  (bind _currentworld_worldasset (break `SoftWorldReference` (`self.CurrentWorld`)))
  (bind _returnvalue_pathstring (`KismetSystemLibrary.BreakSoftObjectPath` (`KismetSystemLibrary.Conv_SoftObjRefToSoftObjPath` _currentworld_worldasset)))
  (set `self.CurrentLevelName` (`.RightS` (`KismetStringLibrary.Split` _returnvalue_pathstring "."))))

(event `self.Box.OnComponentBeginOverlap`
  (params (OverlappedComponent :type "PrimitiveComponent Object Reference") (OtherActor :type "Actor Object Reference") (OtherComp :type "PrimitiveComponent Object Reference") (OtherBodyIndex :type Integer) (bFromSweep :type Boolean) (SweepResult :type "HitResult Structure (by ref)"))
  (bind _currentworld_worldasset (break `SoftWorldReference` (`self.CurrentWorld`)))
  (if (not (`self.Triggered`))
    (bind _asbp_third_person_character (cast `/Game/ThirdPerson/Blueprints/BP_ThirdPersonCharacter` OtherActor))
    (bind _asplayer_game_mode (cast `/Game/GameModes/PlayerGameMode` (`GameplayStatics.GetGameMode`)))
    (bind (_returnvalue_location _returnvalue_rotation _returnvalue_scale) (`KismetMathLibrary.BreakTransform` (`self.GetTransform` _asbp_third_person_character)))
    (set `/Game/GameModes/PlayerGameMode.Respawn Transform` (`KismetMathLibrary.MakeTransform` (`self.K2_GetActorLocation`) _returnvalue_rotation _returnvalue_scale) _asplayer_game_mode)
    (bind _asplayer_game_mode_2 (cast `/Game/GameModes/PlayerGameMode` (`GameplayStatics.GetGameMode`)))
    (set `/Game/GameModes/PlayerGameMode.RespawnLevel` (`self.CurrentWorld`) _asplayer_game_mode_2)
    (set `self.Triggered` true)
    (`|ExecutionSequence`
      (:`then_0`
        (if (`KismetSystemLibrary.IsValidSoftObjectReference` _currentworld_worldasset)
          (bind _outactors (`GameplayStatics.GetAllActorsOfClass` "/Game/Enemy/BP_BaseEnemy.BP_BaseEnemy_C"))
          (set `self.AllEnemies` (`KismetArrayLibrary.Array_Length` _outactors))
          (bind _returnvalue (`KismetSystemLibrary.K2_SetTimerDelegate` (delegate `EnemiesPooling`) 0.033333 true))
          (set `self.Timer` _returnvalue)))
      (:`then_1`
        (`self.Add Tutorial Widget`)))))

(event `EnemiesPooling`
  (if (and (`self.Is Current Level Loaded`) true)
    (bind _outactors (`GameplayStatics.GetAllActorsOfClass` "/Game/Enemy/BP_BaseEnemy.BP_BaseEnemy_C"))
    (set `self.DeadEnemies` 0)
    (for _array_element _outactors
      (if (`/Game/Enemy/BP_BaseEnemy.IsGettingHit` _array_element)
        (`/Engine/EditorBlueprintResources/StandardMacros.IncrementInt` (`self.DeadEnemies`))))
    (if (== (`self.AllEnemies`) (`self.DeadEnemies`))
      (`KismetSystemLibrary.K2_ClearAndInvalidateTimerHandle` (`self.Timer`))
      (bind _asplayer_game_mode (cast `/Game/GameModes/PlayerGameMode` (`GameplayStatics.GetGameMode`)))
      (`/Game/GameModes/PlayerGameMode.SetNextLevel` _asplayer_game_mode (`self.NextWorld`))
      (bind (_direction _newtrack_0) (`Timeline|slowmo` :!via `PlayFromStart`)
        (:`Update`
          (bind _returnvalue (`KismetMathLibrary.Lerp` 1.0 0.05 _newtrack_0))
          (`TimelineComponent.SetPlayRate` (`self.slowmo`) (/ 1.0 _returnvalue))
          (`GameplayStatics.SetGlobalTimeDilation` _returnvalue)
          (set `self.inactive` true))))))

(event `self.ReceiveTick`
  (params (DeltaSeconds :type "Float (single-precision)")))

(fn `Is Current Level Loaded`
  (returns (ReturnValue :type Boolean))
  (return (`LevelStreaming.IsLevelLoaded` (`GameplayStatics.GetStreamingLevel` (`KismetStringLibrary.Conv_StringToName` (`self.CurrentLevelName`))))))

(fn `UserConstructionScript`)