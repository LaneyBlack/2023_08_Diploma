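; Checkpoint actor that sets the player's respawn transform in PlayerGameMode the first time BP_ThirdPersonCharacter overlaps its box.
; On BeginPlay, it line-traces down from the spawn offset to place a safe location above the ground using the player's capsule half-height.
; The Arrow component supplies respawn rotation, and the WasTriggered macro branches on the one-shot flag.
; Tick continually recomputes the spawn offset through transform composition, without updating the safe location.
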(event `self.ReceiveBeginPlay`
  (bind _returnvalue (`GameplayStatics.GetActorOfClass` "/Game/ThirdPerson/Blueprints/BP_ThirdPersonCharacter.BP_ThirdPersonCharacter_C"))
  (set `self.PlayerCapsule` (`CapsuleComponent.GetScaledCapsuleHalfHeight` (`Character.CapsuleComponent` _returnvalue)))
  (set `self.PlayerSafeSpawnLocation` (`self.SanitizeSpawnPosition` (`self.PlayerSpawnLocation`) (`self.K2_GetActorLocation`))))

(event `self.Box.OnComponentBeginOverlap`
  (params (OverlappedComponent :type "PrimitiveComponent Object Reference") (OtherActor :type "Actor Object Reference") (OtherComp :type "PrimitiveComponent Object Reference") (OtherBodyIndex :type Integer) (bFromSweep :type Boolean) (SweepResult :type "HitResult Structure (by ref)"))
  (if (not (`self.Triggered`))
    (bind _asbp_third_person_character (cast `/Game/ThirdPerson/Blueprints/BP_ThirdPersonCharacter` OtherActor))
    (bind _asplayer_game_mode (cast `/Game/GameModes/PlayerGameMode` (`GameplayStatics.GetGameMode`)))
    (bind (_returnvalue_location _returnvalue_rotation _returnvalue_scale) (`KismetMathLibrary.BreakTransform` (`self.GetTransform` _asbp_third_person_character)))
    (set `/Game/GameModes/PlayerGameMode.Respawn Transform` (`KismetMathLibrary.MakeTransform` (`self.PlayerSafeSpawnLocation`) (`SceneComponent.K2_GetComponentRotation` (`self.Arrow`)) _returnvalue_scale) _asplayer_game_mode)
    (set `self.Triggered` true)))

(event `self.ReceiveTick`
  (params (DeltaSeconds :type "Float (single-precision)"))
  (bind _returnvalue (`self.GetTransform`))
  (bind _returnvalue_location (`KismetMathLibrary.BreakTransform` (`KismetMathLibrary.ComposeTransforms` (`KismetMathLibrary.InvertTransform` _returnvalue) (`KismetMathLibrary.MakeTransform` (`self.PlayerSpawnLocation`) (.rotation _returnvalue) (.scale _returnvalue)))))
  (set `self.PlayerSpawnLocation` _returnvalue_location))

(fn `SanitizeSpawnPosition`
  (params (`Check Position` :type "Vector Structure") (ActorLocation :type "Vector Structure"))
  (returns (SanitizedPosition :type "Vector Structure"))
  (locals (NewLocalVar :type "Vector Structure"))
  (bind (_newlocalvar_x _newlocalvar_y) (`KismetMathLibrary.BreakVector` (`local.NewLocalVar`)))
  (bind _output_get (set `local.NewLocalVar` (+ `Check Position` ActorLocation)))
  (bind (_outhit _returnvalue) (`KismetSystemLibrary.LineTraceSingle` _output_get (+ _output_get (0.0 0.0 -2000.0)) "TraceTypeQuery1" true))
  (if _returnvalue
    (return (`KismetMathLibrary.MakeVector` _newlocalvar_x _newlocalvar_y (+ (.z (`.Location` (`GameplayStatics.BreakHitResult` _outhit))) (`self.PlayerCapsule`) 10.0)))))

(fn `UserConstructionScript`)