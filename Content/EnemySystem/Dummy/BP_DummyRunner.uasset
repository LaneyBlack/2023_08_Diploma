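; BP_DummyRunner is a moving test dummy that shows when it takes damage.
; On BeginPlay a slowed Run timeline feeds movement input along the normalized Goal vector, used as a direction rather than a destination.
; Each tick, its static mesh yaws to face the third-person player character.
; ApplyDamage turns its text to a red "DAMAGED", then restores a white "IM GOOD" after a short delay.
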(event `self.ReceiveBeginPlay`
  (`parent.ReceiveBeginPlay`)
  (bind _returnvalue (`GameplayStatics.GetActorOfClass` "/Game/ThirdPerson/Blueprints/BP_ThirdPersonCharacter.BP_ThirdPersonCharacter_C"))
  (set `self.player` _returnvalue)
  (set `self.InitialLocation` (`self.K2_GetActorLocation`))
  (set `self.WorldDirection` (`KismetMathLibrary.Normal` (`self.Goal`)))
  (`TimelineComponent.SetPlayRate` (`self.run`) 0.2)
  (bind (_direction _movementalpha _scalar) (`Timeline|run`)
    (:`Update`
      (`self.AddMovementInput` (`self.WorldDirection`) _scalar))))

(event `self.ReceiveTick`
  (params (DeltaSeconds :type "Float (single-precision)"))
  (bind _player (`self.player`)
    (:`then`
      (bind (_returnvalue_roll _returnvalue_pitch _returnvalue_yaw) (`KismetMathLibrary.BreakRotator` (`KismetMathLibrary.FindLookAtRotation` (`self.K2_GetActorLocation`) (`self.K2_GetActorLocation` _player))))
      (`SceneComponent.K2_SetWorldRotation` (`self.StaticMesh_0`) (`KismetMathLibrary.MakeRotator` 0.0 0.0 _returnvalue_yaw) false false))
    (:`else`)))

(event `self.ApplyDamage`
  (params (PlaneNormal :type "Vector Structure (by ref)") (HitLocation :type "Vector Structure (by ref)"))
  (`TextRenderComponent.K2_SetText` (`self.TextRender`) (`KismetTextLibrary.Conv_NameToText` "DAMAGED"))
  (`TextRenderComponent.SetTextRenderColor` (`self.TextRender`) (make `Color` 0 0 255 255))
  (`KismetSystemLibrary.Delay` 2.0)
  (`TextRenderComponent.K2_SetText` (`self.TextRender`) (`KismetTextLibrary.Conv_NameToText` "IM GOOD"))
  (`TextRenderComponent.SetTextRenderColor` (`self.TextRender`) (make `Color` 255 255 255 255)))

(fn `UserConstructionScript`
  (`parent.UserConstructionScript`))