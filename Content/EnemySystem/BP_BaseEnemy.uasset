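; Base enemy Blueprint with a target-lock widget, one-hit damage and leftover mesh-slicing logic.
; Selection shows the W_Target widget and starts a looping timer that yaws it toward the player.
; ApplyDamage stores the cut plane and nearest bone location, zeroes Health and hides the target frame.
; CovertAndCut slices a procedural copy of the hidden static mesh into physics halves, but its call and the dissolve timeline are disconnected.
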(event `SetMaterials`
  (params (Target :type "MeshComponent Object Reference"))
  ;[1 1 1] Needed for slicing that sucks a dick
)

(event `self.ReceiveBeginPlay`
  (bind _asw_target (cast `/Game/UserInterface/Widgets/Combat/W_Target` (`WidgetComponent.GetWidget` (`self.TargetFrame`))))
  (set `self.As W Target` _asw_target)
  (`SceneComponent.K2_SetRelativeTransform` (`self.StaticMesh`) (`SceneComponent.GetRelativeTransform` (`self.Mesh`)) false false)
  (`SceneComponent.SetVisibility` (`self.StaticMesh`) false false)
  (`self.SetMaterials` null))

(event `self.ApplyDamage`
  (params (PlaneNormal :type "Vector Structure (by ref)") (HitLocation :type "Vector Structure (by ref)"))
  ;[1 1 1 0.497] GetHit
  (set `self.Plane Normal` PlaneNormal)
  (set `self.Hit Location` (`SkinnedMeshComponent.FindClosestBone_K2` (`self.Mesh`) HitLocation 0.0 false))
  (set `self.bIsGettingHit` true)
  (`self.TakeDamage`)
  (`SceneComponent.SetVisibility` (`self.TargetFrame`) false false))

(event `self.SetEnableTargetWidget`
  (params (bIsSelected :type Boolean))
  (bind _targetframe (`self.TargetFrame`))
  (bind (_returnvalue_roll _returnvalue_pitch) (`KismetMathLibrary.BreakRotator` (`SceneComponent.K2_GetComponentRotation` _targetframe)))
  (bind (_returnvalue_roll_2 _returnvalue_pitch_2 _returnvalue_yaw) (`KismetMathLibrary.BreakRotator` (`KismetMathLibrary.FindLookAtRotation` (`self.K2_GetActorLocation`) (`self.K2_GetActorLocation` (`GameplayStatics.GetPlayerCharacter` 0)))))
  (if bIsSelected
    (`KismetSystemLibrary.PrintString` (`KismetStringLibrary.Concat_StrStr` "update widget inside" (`KismetSystemLibrary.GetDisplayName` self)) false)
    (`/Game/UserInterface/Widgets/Combat/W_Target.ShowTarget` (`self.As W Target`))
    ;[1 1 1] Do it with a timer
    (`SceneComponent.K2_SetWorldRotation` _targetframe (`KismetMathLibrary.MakeRotator` _returnvalue_roll _returnvalue_pitch _returnvalue_yaw) false false)
    (bind _returnvalue (`KismetSystemLibrary.K2_SetTimer` null "UpdateWidgetRotation" 0.004167 true))
    (set `self.UpdateWidgetRotationTimer` _returnvalue)
    (else
      (`/Game/UserInterface/Widgets/Combat/W_Target.HideTarget` (`self.As W Target`))
      (`KismetSystemLibrary.K2_ClearAndInvalidateTimerHandle` (`self.UpdateWidgetRotationTimer`)))))

(fn `CovertAndCut`
  (locals (ImpulseStrength :type "Vector Structure"))
  (bind _returnvalue (`self.K2_GetActorLocation`))
  (bind _other_cut_half (`self.Other Cut Half`))
  (bind _proceduralmesh (`self.ProceduralMesh`))
  (bind _plane_normal (`self.Plane Normal`))
  (`SceneComponent.SetVisibility` (`self.Mesh`) false false)
  (`SceneComponent.SetVisibility` (`self.ProceduralMesh`) true false)
  (`KismetProceduralMeshLibrary.CopyProceduralMeshFromStaticMeshComponent` (`self.StaticMesh`) 0 (`self.ProceduralMesh`))
  (set `self.Plane Normal` (* _plane_normal (`KismetMathLibrary.SignOfFloat` (`KismetMathLibrary.Dot_VectorVector` _plane_normal (0.0 0.0 1.0)))))
  (bind _outotherhalfprocmesh (`KismetProceduralMeshLibrary.SliceProceduralMesh` (`self.ProceduralMesh`) (`self.Hit Location`) (`self.Plane Normal`) true "CreateNewSectionForCap" "/Game/DismembermentSystem/m_emissive.m_emissive"))
  (set `self.Other Cut Half` _outotherhalfprocmesh)
  (set `local.ImpulseStrength` (* (`self.GetActorForwardVector`) -10000.0))
  (`PrimitiveComponent.SetSimulatePhysics` _other_cut_half true)
  (`PrimitiveComponent.AddImpulseAtLocation` _other_cut_half (`local.ImpulseStrength`) _returnvalue "None")
  (`PrimitiveComponent.SetSimulatePhysics` _proceduralmesh true)
  (`PrimitiveComponent.AddImpulseAtLocation` _proceduralmesh (`local.ImpulseStrength`) _returnvalue "None"))

(fn `DrawDebugSliceProperties`
  (bind _hit_location (`self.Hit Location`))
  (`KismetSystemLibrary.DrawDebugArrow` _hit_location (+ _hit_location (* (`self.Plane Normal`) 50.0)) 5.0 (struct :`R` 0.855615 :`B` 1.0 :`A` 1.0) 10000.0 2.0)
  (`KismetSystemLibrary.DrawDebugPlane` (`KismetMathLibrary.MakePlaneFromPointAndNormal` (`self.Hit Location`) (`self.Plane Normal`)) (`self.Hit Location`) 100.0 (struct :`G` 0.267682 :`B` 1.0 :`A` 0.5) 1000.0)
  (`KismetSystemLibrary.PrintString` (`KismetStringLibrary.Concat_StrStr` "Hit Location " (`KismetStringLibrary.Conv_VectorToString` (`self.Hit Location`))) true true (struct :`R` 0.082624 :`G` 1.0 :`A` 1.0) 5.0)
  (`KismetSystemLibrary.PrintString` (`KismetStringLibrary.Concat_StrStr` "Plane Normal " (`KismetStringLibrary.Conv_VectorToString` (`self.Plane Normal`))) true true (struct :`R` 0.082624 :`G` 1.0 :`A` 1.0) 5.0))

(fn `TakeDamage`
  (set `self.Health` 0.0))

(fn `UpdateWidgetRotation`
  (bind _targetframe (`self.TargetFrame`))
  (bind (_returnvalue_roll _returnvalue_pitch) (`KismetMathLibrary.BreakRotator` (`SceneComponent.K2_GetComponentRotation` _targetframe)))
  (bind (_returnvalue_roll_2 _returnvalue_pitch_2 _returnvalue_yaw) (`KismetMathLibrary.BreakRotator` (`KismetMathLibrary.FindLookAtRotation` (`self.K2_GetActorLocation`) (`self.K2_GetActorLocation` (`GameplayStatics.GetPlayerCharacter` 0)))))
  (`SceneComponent.K2_SetWorldRotation` _targetframe (`KismetMathLibrary.MakeRotator` _returnvalue_roll _returnvalue_pitch _returnvalue_yaw) false false))

(fn `UserConstructionScript`)