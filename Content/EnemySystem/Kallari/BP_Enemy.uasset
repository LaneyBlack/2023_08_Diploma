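; Enemy character in the Kallari enemy folder that senses the player, attacks, teleports and dies when damage is applied.
; PawnSensing switches the AI_Enemy controller between attacking and passive, while attack events set the HasTouched blackboard key.
; Teleport is a very fast flying AIMoveTo with a selectable particle trail, restoring walking afterward.
; Damage notifies the controller, disables sensing and capsule collision, ragdolls the mesh and increments the kill count.
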(event `self.ReceiveTick`
  (params (DeltaSeconds :type "Float (single-precision)"))
  (`parent.ReceiveTick` DeltaSeconds))

(event `self.ReceiveBeginPlay`
  ;[0.3073 0.3073 0.3073] StartWalkingAround
  (`parent.ReceiveBeginPlay`)
  (set `self.BlackBoardConnectedBinedWithController` (`AIBlueprintHelperLibrary.GetBlackboard` (`AIBlueprintHelperLibrary.GetAIController` self))))

(event `self.ApplyDamage`
  (params (CombatHitData :type "CombatHitData Structure (by ref)"))
  ;[0.2031 0.2031 0.2031] Get Hit
  (`PrimitiveComponent.SetCustomDepthStencilValue` (`self.Mesh`) 0)
  (`GameplayStatics.PlaySoundAtLocation` "/Game/EnemySystem/Sounds/monster-death-grunt-131480.monster-death-grunt-131480" (`self.K2_GetActorLocation` self) (struct) 1.0 1.0 0.0 "/Game/EnemySystem/Sounds/FoodStepsAttenuation.FoodStepsAttenuation" null null null)
  (`parent.ApplyDamage` CombatHitData)
  ;;[0.4792 0.3847 0.2095] turning off Enemy
  (`PawnSensingComponent.SetSensingInterval` (`self.PawnSensing`) 0.0)
  (`SkeletalMeshComponent.SetAnimInstanceClass` (`self.Mesh`) null)
  (bind _asai_enemy (cast `/Game/EnemySystem/Kallari/AI/AI_Enemy` (`self.GetController`)))
  (`/Game/EnemySystem/Kallari/AI/AI_Enemy.Killed` _asai_enemy)
  (`PrimitiveComponent.SetCollisionEnabled` (`self.CapsuleComponent`) "NoCollision")
  (`PrimitiveComponent.SetSimulatePhysics` (`self.Mesh`) true)
  (`ComboSystem.IncreaseKillCount` (`ComboSystem.GetInstance`)))

(event `self.PawnSensing.OnSeePawn`
  (params (Pawn :type "Pawn Object Reference"))
  ;[0.2969 0.2969 0.2969] Tree Behaviour Tasks
  (bind _asai_enemy (cast `/Game/EnemySystem/Kallari/AI/AI_Enemy` (`self.GetController`)))
  (`/Game/EnemySystem/Kallari/AI/AI_Enemy.SetStateAttacking` _asai_enemy Pawn))

(event `self.PawnSensing.OnHearNoise`
  (params (Instigator :type "Pawn Object Reference") (Location :type "Vector Structure (by ref)") (Volume :type "Float (single-precision)"))
  ;[0.2969 0.2969 0.2969] Tree Behaviour Tasks
  (bind _asai_enemy (cast `/Game/EnemySystem/Kallari/AI/AI_Enemy` (`self.GetController`)))
  (`/Game/EnemySystem/Kallari/AI/AI_Enemy.SetStateAttacking` _asai_enemy Instigator))

(event `/Game/EnemySystem/Kallari/AI/BPI_Enemy.CantSeePlayer`
  ;[0.2969 0.2969 0.2969] Tree Behaviour Tasks
  (`KismetSystemLibrary.K2_SetTimer` null "SetCounterCantSeeTo0" 2.0)
  (bind _asai_enemy (cast `/Game/EnemySystem/Kallari/AI/AI_Enemy` (`self.GetController`)))
  (`/Game/EnemySystem/Kallari/AI/AI_Enemy.SetStatePassive` _asai_enemy))

(event `/Game/EnemySystem/Kallari/AI/BPI_Enemy.StartAttack`
  ;[0.2969 0.2969 0.2969] Tree Behaviour Tasks
  (`self.SetBehaviouralTreeBlackboardVariables` true "HasTouched"))

(event `/Game/EnemySystem/Kallari/AI/BPI_Enemy.EndAttack`
  ;[0.2969 0.2969 0.2969] Tree Behaviour Tasks
  (`self.SetBehaviouralTreeBlackboardVariables` false "HasTouched"))

(event `Teleport`
  (params (Location :type "Vector Structure") (attackTarget :type "Actor Object Reference"))
  (bind _charactermovement (`self.CharacterMovement`))
  ;[0.1697 0.3177 0.2923] TELEPORT
  (if (not (`self.IsAttacking`))
    (set `self.IsTeleporting` true)
    (`CharacterMovementComponent.SetMovementMode` _charactermovement "MOVE_Flying" 0)
    (set `CharacterMovementComponent.MaxFlySpeed` 5000.0 _charactermovement)
    (set `CharacterMovementComponent.MaxAcceleration` 999999.0 _charactermovement)
    (switch `/Game/EnemySystem/Kallari/Enumarations/E_EnemyTeleportKind` (`self.EmitterTeleport`)
      (:`NewEnumerator0`
        (set `self.Emitter Template` "/Game/EnemySystem/Kallari/Emitters/P_Countess_TeleportArrive_Emitter1.P_Countess_TeleportArrive_Emitter1"))
      (:`NewEnumerator1`
        (set `self.Emitter Template` "/Game/EnemySystem/Kallari/Emitters/P_Countess_TeleportBegin_Emitter2.P_Countess_TeleportBegin_Emitter2"))
      (:`NewEnumerator2`
        (set `self.Emitter Template` "/Game/EnemySystem/Kallari/Emitters/P_BackJets_Trail_Rogue_Emitter3.P_BackJets_Trail_Rogue_Emitter3"))
      (:`NewEnumerator3`
        (set `self.Emitter Template` "/Game/EnemySystem/Kallari/Emitters/P_Ult_Teleport_Enter_Emitter4.P_Ult_Teleport_Enter_Emitter4"))
      (:`NewEnumerator4`
        (set `self.Emitter Template` "/Game/EnemySystem/Kallari/Emitters/P_Ult_Teleport_Exit_Emitter5.P_Ult_Teleport_Exit_Emitter5")))
    (bind _returnvalue (`GameplayStatics.SpawnEmitterAttached` (`self.Emitter Template`) (`self.Mesh`) "Spine_01" (0.0 0.0 0.0) (struct) (3.0 3.0 3.0)))
    (set `self.TeleportTrail` _returnvalue)
    (`self.StopAnimMontage` null)
    (`|AIMoveTo` self Location attackTarget (`self.RadiusForTeleport`)
      (:`OnSuccess`
        _)
      (:`OnFail`
        _))
    (`self.Teleport End`)
    (else
      (`KismetSystemLibrary.DelayUntilNextTick`)
      (`self.OnTeleportEnd`))))

(event `Teleport End`
  ;[0.1697 0.3177 0.2923] TELEPORT
  (`MovementComponent.StopMovementImmediately` (`self.CharacterMovement`))
  (`CharacterMovementComponent.SetMovementMode` (`self.CharacterMovement`) "MOVE_Walking" 0)
  (set `CharacterMovementComponent.MaxAcceleration` 1500.0 (`self.CharacterMovement`))
  (`self.OnTeleportEnd`)
  (`KismetSystemLibrary.Delay` 0.5)
  (bind _teleporttrail (`self.TeleportTrail`)
    (:`then`
      (`ActorComponent.K2_DestroyComponent` _teleporttrail))
    (:`else`)))

(fn `SetBehaviouralTreeBlackboardVariables`
  (params (BoolValue :type Boolean) (KeyName :type String))
  (bind _blackboardconnectedbinedwithcontroller (`self.BlackBoardConnectedBinedWithController`)
    (:`then`
      (`BlackboardComponent.SetValueAsBool` _blackboardconnectedbinedwithcontroller (`KismetSystemLibrary.MakeLiteralName` (`KismetStringLibrary.Conv_StringToName` KeyName)) BoolValue))
    (:`else`)))

(fn `SetCounterCantSeeTo0`
  (set `self.counterCantSee` 0))

(fn `UserConstructionScript`)