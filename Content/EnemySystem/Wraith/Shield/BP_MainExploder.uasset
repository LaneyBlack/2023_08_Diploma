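; Wraith shield exploder actor that triggers a two-stage explosion by spawning field actors, then destroys itself.
; On BeginPlay it spawns BP_InnerField at its own transform, waits a hard-coded two ticks, then spawns BP_OuterField and destroys itself half a second later.
; CalculateOuterFieldTransform shifts the outer field from the exploder toward the player pawn by OuterOffset.
; Debug prints remain, and a SecondExplosionDelay-to-frames calculation is left unconnected.
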(event `self.ReceiveBeginPlay`
  (`|SpawnActorFromClass` "/Game/EnemySystem/Wraith/Shield/BP_InnerField.BP_InnerField_C" (`self.GetTransform`) "AlwaysSpawn" "MultiplyWithRoot" null null)
  (if (< (`self.TimesDelayed`) 2) :!label _label
    (`KismetSystemLibrary.DelayUntilNextTick`)
    (`/Engine/EditorBlueprintResources/StandardMacros.IncrementInt` (`self.TimesDelayed`)
      (:`  `
        (`KismetSystemLibrary.PrintString` "EXPLOSION DELAYED")
        (goto _label)))
    (else
      (`KismetSystemLibrary.PrintString` "EXPLOSION TRIGGERED")
      (`|SpawnActorFromClass` "/Game/EnemySystem/Wraith/Shield/BP_OuterField.BP_OuterField_C" (`self.CalculateOuterFieldTransform`) "AlwaysSpawn" "MultiplyWithRoot" null null)
      (`KismetSystemLibrary.Delay` 0.5)
      (`self.K2_DestroyActor`))))

(fn `CalculateOuterFieldTransform`
  (returns (ReturnValue :type "Transform Structure (by ref)"))
  (bind (_returnvalue_location _returnvalue_rotation _returnvalue_scale) (`KismetMathLibrary.BreakTransform` (`self.GetTransform`)))
  (return (`KismetMathLibrary.MakeTransform` (+ (`self.K2_GetActorLocation`) (* (`KismetMathLibrary.GetDirectionUnitVector` (`self.K2_GetActorLocation`) (`self.K2_GetActorLocation` (`GameplayStatics.GetPlayerPawn` 0))) (`self.Outer Offset`))) _returnvalue_rotation _returnvalue_scale)))

(fn `UserConstructionScript`)