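; BP_TestExploder is a test actor in the Wraith enemy's shield folder that spawns a pair of field actors when play begins.
; It places BP_InnerField at its own transform and BP_OuterField shifted by OuterOffset along the direction to the first player's pawn.
; The outer field keeps the exploder's rotation and scale, and both always spawn regardless of collision.
; The player direction is sampled once, with no later update.
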(event `self.ReceiveBeginPlay`
  (`|SpawnActorFromClass` "/Game/EnemySystem/Wraith/Shield/BP_InnerField.BP_InnerField_C" (`self.GetTransform`) "AlwaysSpawn" "MultiplyWithRoot" null null)
  (`|SpawnActorFromClass` "/Game/EnemySystem/Wraith/Shield/BP_OuterField.BP_OuterField_C" (`self.CalculateOuterFieldTransform`) "AlwaysSpawn" "MultiplyWithRoot" null null))

(fn `CalculateOuterFieldTransform`
  (returns (ReturnValue :type "Transform Structure (by ref)"))
  (bind (_returnvalue_location _returnvalue_rotation _returnvalue_scale) (`KismetMathLibrary.BreakTransform` (`self.GetTransform`)))
  (return (`KismetMathLibrary.MakeTransform` (+ (`self.K2_GetActorLocation`) (* (`KismetMathLibrary.GetDirectionUnitVector` (`self.K2_GetActorLocation`) (`self.K2_GetActorLocation` (`GameplayStatics.GetPlayerPawn` 0))) (`self.Outer Offset`))) _returnvalue_rotation _returnvalue_scale)))

(fn `UserConstructionScript`)