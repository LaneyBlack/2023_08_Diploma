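; Bullet pool for a BP_RangedEnemy owner, pre-creating the enemy's bullets instead of spawning them on demand.
; On BeginPlay it copies the owner's BulletKind and spawns a set number of BP_Bullet actors into the pool array.
; Each bullet's OnBulletDestroyed event teleports it back to the spawn location for reuse.
; DestroyAllBullets destroys every pooled bullet; firing logic is not handled here.
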(event `self.ReceiveBeginPlay`
  ;[1 1 1] BulletKind
  (bind _asbp_ranged_enemy (cast `/Game/EnemySystem/Wraith/BP_RangedEnemy` (`self.GetOwner`)))
  (set `self.BulletKind` (`/Game/EnemySystem/Wraith/BP_RangedEnemy.BulletKind` _asbp_ranged_enemy))
  ;[1 1 1] Create Bullets
  (for _ (range (+ (`self.AmountOfBullets`) 1))
    (bind _returnvalue (`|SpawnActorFromClass` "/Game/EnemySystem/Wraith/Shooting/BP_Bullet.BP_Bullet_C" (`KismetMathLibrary.MakeTransform` (`self.SpawnLocation`)) "Undefined" "MultiplyWithRoot" (`self.GetOwner`) (`self.BulletKind`) null))
    (add `/Game/EnemySystem/Wraith/Shooting/BP_Bullet.OnBulletDestroyed` _returnvalue (delegate `ReturnToBullet`))
    (`KismetArrayLibrary.Array_Add` (`self.BulletPool`) _returnvalue)))

(event `ReturnToBullet`
  (params (Bullet :type "/Game/EnemySystem/Wraith/Shooting/BP_Bullet Object Reference"))
  ;[1 1 1] Create Bullets
  (`/Engine/EditorBlueprintResources/StandardMacros.IsValid` Bullet
    (:`Is Valid`
      (`Actor.K2_SetActorLocation` Bullet (`self.SpawnLocation`) false false))))

(event `DestroyAllBullets`
  ;[1 1 1] Destroy Bullets
  (for _array_element (`self.BulletPool`)
    (`Actor.K2_DestroyActor` _array_element)))