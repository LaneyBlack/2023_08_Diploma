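; BP_BulletPool is an object pool that pre-spawns BP_Bullet actors for its owner, filed under the Wraith enemy's shooting assets.
; On BeginPlay it spawns the bullets at SpawnLocation, makes their collision spheres ignore the owner when moving, and stores them in BulletPool.
; Each bullet's OnBulletDestroyed event moves it back to SpawnLocation instead of spawning a replacement.
; DestroyAllBullets destroys every pooled actor.
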(event `self.ReceiveBeginPlay`
  (for _ (range (+ (`self.AmountOfBullets`) 1))
    (bind _returnvalue (`|SpawnActorFromClass` "/Game/Enemy/Wraith/Shooting/BP_Bullet.BP_Bullet_C" (`KismetMathLibrary.MakeTransform` (`self.SpawnLocation`)) "Undefined" "MultiplyWithRoot" (`self.GetOwner`) null))
    (add `/Game/Enemy/Wraith/Shooting/BP_Bullet.OnBulletDestroyed` _returnvalue (delegate `ReturnToBullet`))
    (`PrimitiveComponent.IgnoreActorWhenMoving` (`/Game/Enemy/Wraith/Shooting/BP_Bullet.Sphere` _returnvalue) (`self.GetOwner`) true)
    (`KismetArrayLibrary.Array_Add` (`self.BulletPool`) _returnvalue)))

(event `ReturnToBullet`
  (params (Bullet :type "/Game/Enemy/Wraith/Shooting/BP_Bullet Object Reference"))
  (`/Engine/EditorBlueprintResources/StandardMacros.IsValid` Bullet
    (:`Is Valid`
      (`Actor.K2_SetActorLocation` Bullet (`self.SpawnLocation`) false false))))

(event `DestroyAllBullets`
  (for _array_element (`self.BulletPool`)
    (`Actor.K2_DestroyActor` _array_element)))