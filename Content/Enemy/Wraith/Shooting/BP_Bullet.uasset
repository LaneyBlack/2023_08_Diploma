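; Reusable enemy projectile that fires from its owner at the player's aim socket and can be parried back at the shooter.
; A hit damages the player or enemy, then deactivates the bullet and calls OnBulletDestroyed, as does a lifetime timer.
; Entering ParryWindow slows time and starts timer polling of CombatSystemComponent for a fresh parry press.
; A successful parry triggers the perfect-parry response, retargets the bullet and enlarges its collision.
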(event `self.ReceiveBeginPlay`
  ;[1 1 1] Start
  (set `self.PlayerIsTarget` true))

(event `self.Sphere.OnComponentHit`
  (params (HitComponent :type "PrimitiveComponent Object Reference") (OtherActor :type "Actor Object Reference") (OtherComp :type "PrimitiveComponent Object Reference") (NormalImpulse :type "Vector Structure") (Hit :type "HitResult Structure (by ref)"))
  ;[0.5 1 1 0.403] On collision
  (`self.PrintObject` OtherActor "Actor")
  (`self.PrintObject` OtherComp "Component")
  (`self.HandleImpact` Hit)
  (`ActorComponent.Deactivate` (`self.ProjectileMovement`))
  (`|ExecutionSequence`
    (:`then_0`
      (if (`self.PlayerIsTarget`)
        (bind _asbp_third_person_character (cast `/Game/ThirdPerson/Blueprints/BP_ThirdPersonCharacter` OtherActor))
        (`KismetSystemLibrary.PrintString` "PLAYER DAMAGED" true true (struct :`R` 1.0 :`B` 0.270337 :`A` 1.0))
        (`GameplayStatics.ApplyDamage` _asbp_third_person_character 100.0)
        (set `self.AlreadyHit` true :!label _label)
        (`self.DeactivateBullet`)
        (`self.OnBulletDestroyed` self)))
    (:`then_1`
      (bind _asbase_enemy (cast `BaseEnemy` OtherActor))
      (if (or (not (`self.PlayerIsTarget`)) (!= OtherActor (`self.GetOwner`)))
        (`BaseEnemy.ApplyDamage` _asbase_enemy)
        (goto _label)))
    (:`then_2`
      (`/Engine/EditorBlueprintResources/StandardMacros.IsValid` HitComponent
        (:`Is Valid`
          (goto _label))))))

(event `FireBullet`
  (`ActorComponent.Activate` (`self.ProjectileMovement`) true)
  (bind _returnvalue (`self.GetSpawnLocation`))
  (`self.K2_SetActorLocation` _returnvalue)
  ;[0.5 1 1 0.346] If nothing touches
  (set `self.AlreadyHit` false)
  (`KismetSystemLibrary.K2_SetTimerDelegate` (delegate `ResetBullet`) 5.0)
  ;[1 1 1 0.335] BulletEvents
  (bind _velocity (`self.SetBulletVelocity`))
  (set `self.PlayerIsTarget` true)
  (set `MovementComponent.Velocity` _velocity (`self.ProjectileMovement`))
  (`KismetSystemLibrary.K2_ClearAndInvalidateTimerHandle` (`self.ParryPoolingTimer`) :!label _label_2)
  (`SphereComponent.SetSphereRadius` (`self.Sphere`) (`self.SphereCollisionRadius`) true)
  (`self.HandleParryState` true))

(event `ResetBullet`
  ;[0.5 1 1 0.346] If nothing touches
  (if (not (`self.AlreadyHit`))
    (`self.DeactivateBullet`)
    (`self.OnBulletDestroyed` self)))

(event `DeactivateBullet`
  ;[1 1 1 0.335] BulletEvents
  (set `self.AlreadyHit` true)
  (`/Engine/EditorBlueprintResources/StandardMacros.IsValid` (`self.Sphere`)
    (:`Is Valid`
      (set `self.PlayerIsTarget` true)
      (`MovementComponent.StopMovementImmediately` (`self.ProjectileMovement`))
      (goto _label_2))))

(event `self.ParryWindow.OnComponentBeginOverlap`
  (params (OverlappedComponent :type "PrimitiveComponent Object Reference") (OtherActor :type "Actor Object Reference") (OtherComp :type "PrimitiveComponent Object Reference") (OtherBodyIndex :type Integer) (bFromSweep :type Boolean) (SweepResult :type "HitResult Structure (by ref)"))
  ;[0.429 0.3085 0.1784] Parrying
  (if (`self.PlayerIsTarget`)
    (bind _asbp_third_person_character (cast `/Game/ThirdPerson/Blueprints/BP_ThirdPersonCharacter` OtherActor))
    (bind _output_get (set `self.Combat System Component` (`TheFallenSamuraiCharacter.CombatSystemComponent` _asbp_third_person_character)))
    (`/Engine/EditorBlueprintResources/StandardMacros.IsValid` _output_get
      (:`Is Valid`
        (`self.HandleParryState` false)
        (set `self.ParryLastFrame` (`CombatSystemComponent.bInParry` _output_get))
        (bind _returnvalue (`KismetSystemLibrary.K2_SetTimer` null "ParryPooling" 0.016667 true))
        (set `self.ParryPoolingTimer` _returnvalue)
        (bind _asbp_ranged_enemy (cast `/Game/Enemy/Wraith/BP_RangedEnemy` (`self.GetOwner`)))
        (`/Game/Enemy/BP_BaseEnemy.ParryEvent` _asbp_ranged_enemy)))))

(event `self.ParryWindow.OnComponentEndOverlap`
  (params (OverlappedComponent :type "PrimitiveComponent Object Reference") (OtherActor :type "Actor Object Reference") (OtherComp :type "PrimitiveComponent Object Reference") (OtherBodyIndex :type Integer))
  (cast `/Game/ThirdPerson/Blueprints/BP_ThirdPersonCharacter` OtherActor)
  (`self.HandleParryState` true)
  (`KismetSystemLibrary.K2_ClearAndInvalidateTimerHandle` (`self.ParryPoolingTimer`)))

(event `self.ReceiveTick`
  (params (DeltaSeconds :type "Float (single-precision)"))
  (`KismetSystemLibrary.PrintString` (`KismetStringLibrary.Concat_StrStr` "Bullet(" (`KismetSystemLibrary.GetDisplayName` self) ") player is target = " (`KismetStringLibrary.Conv_BoolToString` (`self.PlayerIsTarget`))) false true (struct :`G` 0.66 :`B` 1.0 :`A` 1.0) 0.0))

(event `self.ParryWindowWindup.OnComponentBeginOverlap`
  (params (OverlappedComponent :type "PrimitiveComponent Object Reference") (OtherActor :type "Actor Object Reference") (OtherComp :type "PrimitiveComponent Object Reference") (OtherBodyIndex :type Integer) (bFromSweep :type Boolean) (SweepResult :type "HitResult Structure (by ref)"))
  (if (`self.PlayerIsTarget`)
    (cast `/Game/ThirdPerson/Blueprints/BP_ThirdPersonCharacter` OtherActor)
    (`NiagaraFunctionLibrary.SpawnSystemAttached` "/Game/Explosions_W3Vol1/Niagara/NS_Burst1.NS_Burst1" (`self.BulletPE`) "None" (0.0 0.0 0.0) (struct) "KeepRelativeOffset")))

(fn `GetDeflectionVelocity`
  (params (`Deflect Speed` :type "Float (double-precision)"))
  (returns (Velocity :type "Vector Structure"))
  (return (* (`KismetMathLibrary.Normal` (- (`self.K2_GetActorLocation` (`self.GetOwner`)) (`self.K2_GetActorLocation` (`ActorComponent.GetOwner` (`self.Combat System Component`))))) (`local.Deflect Speed`))))

(fn `GetSpawnLocation`
  (returns (ReturnValue :type "Vector Structure"))
  (return (+ (`self.K2_GetActorLocation` (`self.GetOwner`)) (0.0 0.0 50.0))))

(fn `HandleImpact`
  (params (HitResult :type "HitResult Structure"))
  (`GameplayStatics.SpawnEmitterAtLocation` "/Game/AdvancedMagicFX12/particles/P_ky_hit_water.P_ky_hit_water" (`.ImpactPoint` (`GameplayStatics.BreakHitResult` HitResult)) (struct) (0.3 0.3 0.3)))

(fn `HandleParryState`
  (params (Reset :type Boolean))
  (`KismetSystemLibrary.PrintString` "Hello")
  (`SceneComponent.SetVisibility` (`self.BulletPE`) Reset false)
  (`SceneComponent.SetVisibility` (`self.ParriedBulletPE`) (not Reset) false)
  (`GameplayStatics.SetGlobalTimeDilation` (`KismetMathLibrary.SelectFloat` 1.0 0.6 (`local.Reset`))))

(fn `MakeSound`
  ;[1 1 1] w bulletcie
  (switch `int` (`KismetMathLibrary.RandomIntegerInRange` 0 1)
    (:`0`
      (`GameplayStatics.PlaySoundAtLocation` "/Game/Enemy/Sounds/metal1.metal1" (`self.K2_GetActorLocation` self) (struct) 1.0 1.0 0.0 "/Game/Enemy/Sounds/FoodStepsAttenuation.FoodStepsAttenuation" null null null))
    (:`1`
      (`GameplayStatics.PlaySoundAtLocation` "/Game/Enemy/Sounds/metal2.metal2" (`self.K2_GetActorLocation` self) (struct) 1.0 1.0 0.0 "/Game/Enemy/Sounds/FoodStepsAttenuation.FoodStepsAttenuation" null null null))))

(fn `ParryPooling`
  (bind _velocity (`self.GetDeflectionVelocity` 10000.0))
  (`KismetSystemLibrary.PrintString` (`KismetStringLibrary.Concat_StrStr` "parry pooling by " (`KismetSystemLibrary.GetDisplayName` self)) false true (struct :`R` 0.162671 :`G` 0.95 :`A` 1.0) 5.0)
  (`/Engine/EditorBlueprintResources/StandardMacros.IsValid` (`self.Combat System Component`)
    (:`Is Valid`
      (if (and (not (`self.ParryLastFrame`)) (`CombatSystemComponent.bInParry` (`self.Combat System Component`)))
        (set `MovementComponent.Velocity` (0.0 0.0 0.0) (`self.ProjectileMovement`))
        (`KismetSystemLibrary.PrintString` (`KismetStringLibrary.Concat_StrStr` "POOLING STOPED BY" (`KismetSystemLibrary.GetDisplayName` self)) false true (struct :`R` 0.99 :`A` 1.0) 5.0)
        (`KismetSystemLibrary.K2_ClearAndInvalidateTimerHandle` (`self.ParryPoolingTimer`))
        (bind _asbp_base_enemy (cast `/Game/Enemy/BP_BaseEnemy` (`self.GetOwner`)))
        (`CombatSystemComponent.PerfectParryResponse` (`self.Combat System Component`) (`KismetMathLibrary.SelectInt` 0 1 (`/Game/Enemy/BP_BaseEnemy.Was Parried` _asbp_base_enemy)) true)
        (set `/Game/Enemy/BP_BaseEnemy.Was Parried` true _asbp_base_enemy)
        (set `self.DeflectedDirection` _velocity)
        (set `MovementComponent.Velocity` _velocity (`self.ProjectileMovement`))
        (set `self.PlayerIsTarget` false)
        (`PrimitiveComponent.IgnoreActorWhenMoving` (`self.Sphere`) (`self.GetOwner`) false)
        (`SphereComponent.SetSphereRadius` (`self.Sphere`) 60.0 true)
        (bind _asbp_ranged_enemy (cast `/Game/Enemy/Wraith/BP_RangedEnemy` (`self.GetOwner`)))
        (`/Game/Enemy/BP_BaseEnemy.SuccessfulParryEvent` _asbp_ranged_enemy)
        (`self.MakeSound`)
        (else
          (set `self.ParryLastFrame` (`CombatSystemComponent.bInParry` (`self.Combat System Component`))))))))

(fn `PrintObject`
  (params (Object :type "Object Object Reference") (Name :type String))
  (`KismetSystemLibrary.PrintString` (`KismetStringLibrary.Concat_StrStr` Name " hit name = " (`KismetSystemLibrary.GetDisplayName` Object))))

(fn `SetBulletVelocity`
  (returns (Velocity :type "Vector Structure"))
  (return (* (`KismetMathLibrary.GetDirectionUnitVector` (`self.K2_GetActorLocation` (`self.GetOwner`)) (`SceneComponent.GetSocketLocation` (`Character.Mesh` (`GameplayStatics.GetPlayerCharacter` 0)) "AimTarget")) (`ProjectileMovementComponent.InitialSpeed` (`self.ProjectileMovement`)))))

(fn `SetHidden`
  (params (`Is Hidden` :type Boolean))
  (`SceneComponent.SetHiddenInGame` (`self.Sphere`) `Is Hidden` true)
  (`SceneComponent.SetHiddenInGame` (`self.BulletMesh`) true false))

(fn `UserConstructionScript`)