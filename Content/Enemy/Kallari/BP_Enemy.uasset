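; Enemy character Blueprint that senses targets, attacks, and dies from a hit.
; PawnSensing sight and hearing switch the AI_Enemy controller to attacking, CantSeePlayer returns it to passive, and attack start/end events toggle the HasTouched blackboard key.
; ApplyDamage plays a death grunt, passes hit plane and location to the parent, notifies the controller, ragdolls the mesh without capsule collision, and increments the game instance kill count.
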(event `self.ReceiveBeginPlay`
  ;[0.3073 0.3073 0.3073] StartWalkingAround
  (`parent.ReceiveBeginPlay`)
  (set `self.BlackBoardConnectedBinedWithController` (`AIBlueprintHelperLibrary.GetBlackboard` (`AIBlueprintHelperLibrary.GetAIController` self))))

(event `self.ApplyDamage`
  (params (PlaneNormal :type "Vector Structure (by ref)") (HitLocation :type "Vector Structure (by ref)"))
  ;[0.2031 0.2031 0.2031] Get Hit
  (`PrimitiveComponent.SetCustomDepthStencilValue` (`self.Mesh`) 0)
  (`GameplayStatics.PlaySoundAtLocation` "/Game/Enemy/Sounds/monster-death-grunt-131480.monster-death-grunt-131480" (`self.K2_GetActorLocation` self) (struct) 1.0 1.0 0.0 "/Game/Enemy/Sounds/FoodStepsAttenuation.FoodStepsAttenuation" null null null)
  (`parent.ApplyDamage` PlaneNormal HitLocation)
  ;;[0.4792 0.3847 0.2095] turning off Enemy
  (`PawnSensingComponent.SetSensingInterval` (`self.PawnSensing`) 0.0)
  (`SkeletalMeshComponent.SetAnimInstanceClass` (`self.Mesh`) null)
  (bind _asai_enemy (cast `/Game/Enemy/Kallari/AI/AI_Enemy` (`self.GetController`)))
  (`/Game/Enemy/Kallari/AI/AI_Enemy.Killed` _asai_enemy)
  (`PrimitiveComponent.SetCollisionEnabled` (`self.CapsuleComponent`) "NoCollision")
  (`PrimitiveComponent.SetSimulatePhysics` (`self.Mesh`) true)
  (`ComboSystem.IncreaseKillCount` (`ComboSystem.GetInstance`)))

(event `self.PawnSensing.OnSeePawn`
  (params (Pawn :type "Pawn Object Reference"))
  ;[0.2969 0.2969 0.2969] Tree Behaviour Tasks
  (bind _asai_enemy (cast `/Game/Enemy/Kallari/AI/AI_Enemy` (`self.GetController`)))
  (`/Game/Enemy/Kallari/AI/AI_Enemy.SetStateAttacking` _asai_enemy Pawn))

(event `self.PawnSensing.OnHearNoise`
  (params (Instigator :type "Pawn Object Reference") (Location :type "Vector Structure (by ref)") (Volume :type "Float (single-precision)"))
  ;[0.2969 0.2969 0.2969] Tree Behaviour Tasks
  (bind _asai_enemy (cast `/Game/Enemy/Kallari/AI/AI_Enemy` (`self.GetController`)))
  (`/Game/Enemy/Kallari/AI/AI_Enemy.SetStateAttacking` _asai_enemy Instigator))

(event `/Game/Enemy/Kallari/AI/BPI_Enemy.CantSeePlayer`
  ;[0.2969 0.2969 0.2969] Tree Behaviour Tasks
  (bind _asai_enemy (cast `/Game/Enemy/Kallari/AI/AI_Enemy` (`self.GetController`)))
  (`/Game/Enemy/Kallari/AI/AI_Enemy.SetStatePassive` _asai_enemy))

(event `/Game/Enemy/Kallari/AI/BPI_Enemy.StartAttack`
  ;[0.2969 0.2969 0.2969] Tree Behaviour Tasks
  (`self.SetBehaviouralTreeBlackboardVariables` true "HasTouched"))

(event `/Game/Enemy/Kallari/AI/BPI_Enemy.EndAttack`
  ;[0.2969 0.2969 0.2969] Tree Behaviour Tasks
  (`self.SetBehaviouralTreeBlackboardVariables` false "HasTouched"))

(event `self.ReceiveTick`
  (params (DeltaSeconds :type "Float (single-precision)"))
  (`parent.ReceiveTick` DeltaSeconds))

(fn `SetBehaviouralTreeBlackboardVariables`
  (params (BoolValue :type Boolean) (KeyName :type String))
  (bind _blackboardconnectedbinedwithcontroller (`self.BlackBoardConnectedBinedWithController`)
    (:`then`
      (`BlackboardComponent.SetValueAsBool` _blackboardconnectedbinedwithcontroller (`KismetSystemLibrary.MakeLiteralName` (`KismetStringLibrary.Conv_StringToName` KeyName)) BoolValue))
    (:`else`)))

(fn `UserConstructionScript`)