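; BP_DummyRunner is a test dummy character that runs along the direction of its Goal vector.
; On BeginPlay it plays the slowed Run timeline, whose Scalar track scales movement input along the normalized Goal.
; Tick yaws its TextRender toward the third-person player character.
; ApplyDamage only prints a log message, and SetDebugTextValue is empty, with its text update left disconnected.
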(event `self.ReceiveBeginPlay`
  (`parent.ReceiveBeginPlay`)
  (bind _returnvalue (`GameplayStatics.GetActorOfClass` "/Game/ThirdPerson/Blueprints/BP_ThirdPersonCharacter.BP_ThirdPersonCharacter_C"))
  (set `self.player` _returnvalue)
  (set `self.InitialLocation` (`self.K2_GetActorLocation`))
  (set `self.WorldDirection` (`KismetMathLibrary.Normal` (`self.Goal`)))
  (`TimelineComponent.SetPlayRate` (`self.run`) 0.2)
  (bind (_direction _movementalpha _scalar) (`Timeline|run`)
    (:`Update`
      (`self.AddMovementInput` (`self.WorldDirection`) _scalar))))

(event `self.ReceiveTick`
  (params (DeltaSeconds :type "Float (single-precision)"))
  (bind _player (`self.player`)
    (:`then`
      (bind (_returnvalue_roll _returnvalue_pitch _returnvalue_yaw) (`KismetMathLibrary.BreakRotator` (`KismetMathLibrary.FindLookAtRotation` (`self.K2_GetActorLocation`) (`self.K2_GetActorLocation` _player))))
      (`SceneComponent.K2_SetRelativeRotation` (`self.TextRender`) (`KismetMathLibrary.MakeRotator` 0.0 0.0 _returnvalue_yaw) false false))
    (:`else`)))

(event `self.ApplyDamage`
  (`KismetSystemLibrary.PrintString` "DAMAGE" false true (struct :`R` 0.91 :`A` 1.0)))

(event `self.SetDebugTextValue`
  (params (value :type String)))

(fn `UserConstructionScript`
  (`parent.UserConstructionScript`))