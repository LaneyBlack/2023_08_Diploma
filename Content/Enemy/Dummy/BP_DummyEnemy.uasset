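; BP_DummyEnemy is a dummy enemy that displays a numeric debug value on a text render above or on itself.
; On BeginPlay it caches the third-person character, then each tick yaws the text render to face that player.
; SetDebugTextValue writes a number to the text, while ApplyDamage only logs a DAMAGE string without showing it on screen or changing any health.
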(event `self.ReceiveBeginPlay`
  (bind _returnvalue (`GameplayStatics.GetActorOfClass` "/Game/ThirdPerson/Blueprints/BP_ThirdPersonCharacter.BP_ThirdPersonCharacter_C"))
  (set `self.player` _returnvalue))

(event `self.ReceiveTick`
  (params (DeltaSeconds :type "Float (single-precision)"))
  (bind _player (`self.player`)
    (:`then`
      (bind (_returnvalue_roll _returnvalue_pitch _returnvalue_yaw) (`KismetMathLibrary.BreakRotator` (`KismetMathLibrary.FindLookAtRotation` (`self.K2_GetActorLocation`) (`self.K2_GetActorLocation` _player))))
      (`SceneComponent.K2_SetRelativeRotation` (`self.TextRender`) (`KismetMathLibrary.MakeRotator` 0.0 0.0 _returnvalue_yaw) false false))
    (:`else`)))

(event `self.ApplyDamage`
  (`KismetSystemLibrary.PrintString` "DAMAGE" false true (struct :`R` 0.91 :`A` 1.0)))

(event `self.SetDebugTextValue`
  (params (value :type "Float (single-precision)"))
  (`TextRenderComponent.K2_SetText` (`self.TextRender`) (`KismetTextLibrary.Conv_DoubleToText` value "HalfToEven")))

(fn `UserConstructionScript`
  (`parent.UserConstructionScript`))