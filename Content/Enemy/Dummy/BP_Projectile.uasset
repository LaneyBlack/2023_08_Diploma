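; BP_Projectile is a projectile that damages what it overlaps and can be perfect-parried by the player.
; While targeting the player, its ParryWindow starts a fast looping timer that polls CombatSystemComponent for a fresh parry press.
; A parry triggers the perfect-parry response and relaunches it faster along the player's forward vector, no longer targeting them.
; DamageCollision always damages overlapped BaseEnemy actors and destroys the projectile on a hit.
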(event `self.DamageCollision.OnComponentBeginOverlap`
  (params (OverlappedComponent :type "PrimitiveComponent Object Reference") (OtherActor :type "Actor Object Reference") (OtherComp :type "PrimitiveComponent Object Reference") (OtherBodyIndex :type Integer) (bFromSweep :type Boolean) (SweepResult :type "HitResult Structure (by ref)"))
  (`|ExecutionSequence`
    (:`then_0`
      (if (`self.PlayerIsTarget`)
        (`GameplayStatics.ApplyDamage` OtherActor 1000.0)))
    (:`then_1`
      (bind _asbase_enemy (cast `BaseEnemy` OtherActor))
      (`BaseEnemy.ApplyDamage` _asbase_enemy))))

(event `self.ParryWindow.OnComponentBeginOverlap`
  (params (OverlappedComponent :type "PrimitiveComponent Object Reference") (OtherActor :type "Actor Object Reference") (OtherComp :type "PrimitiveComponent Object Reference") (OtherBodyIndex :type Integer) (bFromSweep :type Boolean) (SweepResult :type "HitResult Structure (by ref)"))
  (if (`self.PlayerIsTarget`)
    (bind _asbp_third_person_character (cast `/Game/ThirdPerson/Blueprints/BP_ThirdPersonCharacter` OtherActor))
    (`/Engine/EditorBlueprintResources/StandardMacros.DoOnce` false
      (:`Completed`
        (bind _output_get (set `self.Combat System Component` (`TheFallenSamuraiCharacter.CombatSystemComponent` _asbp_third_person_character)))
        (`/Engine/EditorBlueprintResources/StandardMacros.IsValid` _output_get
          (:`Is Valid`
            (set `self.ParryLastFrame` (`CombatSystemComponent.bInParry` _output_get))
            (bind _returnvalue (`KismetSystemLibrary.K2_SetTimer` null "ParryPooling" 0.008333 true))
            (set `self.ParryPoolingTimer` _returnvalue)))))))

(event `self.DamageCollision.OnComponentHit`
  (params (HitComponent :type "PrimitiveComponent Object Reference") (OtherActor :type "Actor Object Reference") (OtherComp :type "PrimitiveComponent Object Reference") (NormalImpulse :type "Vector Structure") (Hit :type "HitResult Structure (by ref)"))
  (`self.K2_DestroyActor`))

(event `self.ParryWindow.OnComponentEndOverlap`
  (params (OverlappedComponent :type "PrimitiveComponent Object Reference") (OtherActor :type "Actor Object Reference") (OtherComp :type "PrimitiveComponent Object Reference") (OtherBodyIndex :type Integer))
  (`KismetSystemLibrary.K2_ClearAndInvalidateTimerHandle` (`self.ParryPoolingTimer`)))

(fn `ParryPooling`
  (bind _returnvalue (`self.GetActorForwardVector` (`ActorComponent.GetOwner` (`self.Combat System Component`))))
  (`KismetSystemLibrary.PrintString` (`KismetStringLibrary.Concat_StrStr` "parry pooling by " (`KismetSystemLibrary.GetDisplayName` self)) false true (struct :`R` 0.162671 :`G` 0.95 :`A` 1.0) 5.0)
  (`/Engine/EditorBlueprintResources/StandardMacros.IsValid` (`self.Combat System Component`)
    (:`Is Valid`
      (if (and (not (`self.ParryLastFrame`)) (`CombatSystemComponent.bInParry` (`self.Combat System Component`)))
        (`KismetSystemLibrary.PrintString` (`KismetStringLibrary.Concat_StrStr` "POOLING STOPED BY" (`KismetSystemLibrary.GetDisplayName` self)) false true (struct :`R` 0.99 :`A` 1.0) 5.0)
        (`KismetSystemLibrary.K2_ClearAndInvalidateTimerHandle` (`self.ParryPoolingTimer`))
        (`CombatSystemComponent.PerfectParryResponse` (`self.Combat System Component`) 0 false)
        (set `self.DeflectedDirection` _returnvalue)
        (set `MovementComponent.Velocity` (* _returnvalue (`ProjectileMovementComponent.InitialSpeed` (`self.ProjectileMovement`)) 5.0) (`self.ProjectileMovement`))
        (set `self.PlayerIsTarget` false)
        (else
          (set `self.ParryLastFrame` (`CombatSystemComponent.bInParry` (`self.Combat System Component`))))))))

(fn `UserConstructionScript`)