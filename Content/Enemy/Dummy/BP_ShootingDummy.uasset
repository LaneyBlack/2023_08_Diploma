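; BP_ShootingDummy is a dummy enemy that fires projectiles and displays a reaction when damaged.
; A Delay on Tick acts as a repeating timer, spawning a BP_Projectile in front of the actor every few seconds at TravelSpeed.
; The ApplyDamage event turns the TextRender into a red damage notice, then switches it to a white all-clear message after a short delay.
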(event `self.ReceiveTick`
  (params (DeltaSeconds :type "Float (single-precision)"))
  (`KismetSystemLibrary.Delay` 2.5)
  (bind _returnvalue (`|SpawnActorFromClass` "/Game/Enemy/Dummy/BP_Projectile.BP_Projectile_C" (`KismetMathLibrary.MakeTransform` (+ (`self.K2_GetActorLocation`) (* (`self.GetActorForwardVector`) 100.0))) "AlwaysSpawn" "MultiplyWithRoot" null null))
  (bind _projectilemovement (`/Game/Enemy/Dummy/BP_Projectile.ProjectileMovement` _returnvalue))
  (bind _output_get (set `ProjectileMovementComponent.InitialSpeed` (`self.TravelSpeed`) _projectilemovement))
  (set `ProjectileMovementComponent.MaxSpeed` _output_get _projectilemovement))

(event `self.ApplyDamage`
  (`TextRenderComponent.K2_SetText` (`self.TextRender`) (`KismetTextLibrary.Conv_NameToText` "DAMAGED"))
  (`TextRenderComponent.SetTextRenderColor` (`self.TextRender`) (make `Color` 0 0 1 1))
  (`KismetSystemLibrary.Delay` 2.0)
  (`TextRenderComponent.K2_SetText` (`self.TextRender`) (`KismetTextLibrary.Conv_NameToText` "IM GOOD"))
  (`TextRenderComponent.SetTextRenderColor` (`self.TextRender`) (make `Color` 1 1 1 1)))

(fn `UserConstructionScript`
  (`parent.UserConstructionScript`))