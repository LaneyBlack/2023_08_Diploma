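; Base enemy Blueprint that shows world-space target frame and parry icon widgets for player combat.
; Selection shows the target frame and starts a fast looping timer that yaws it toward the player, cleared on deselection.
; Tick continuously turns the parry icon toward the player and deactivates it once the enemy has been parried.
; ApplyDamage flags the hit, sets health straight to zero and hides both widgets.
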(event `self.ReceiveBeginPlay`
  (bind _asw_target (cast `/Game/UserInterface/Widgets/Combat/W_Target` (`WidgetComponent.GetWidget` (`self.TargetFrame`))))
  (set `self.As W Target` _asw_target)
  (bind _asw_parry_icon (cast `/Game/UserInterface/Widgets/Combat/W_ParryIcon` (`WidgetComponent.GetWidget` (`self.Parry`))))
  (bind _output_get (set `self.As W Parry Icon` _asw_parry_icon))
  (`/Game/UserInterface/Widgets/Combat/W_ParryIcon.SetActive` _output_get true))

(event `self.ApplyDamage`
  ;[1 1 1 0.497] GetHit
  (set `self.bIsGettingHit` true)
  (`self.TakeDamage`)
  (`SceneComponent.SetVisibility` (`self.TargetFrame`) false false)
  (`SceneComponent.SetVisibility` (`self.Parry`) false false))

(event `self.SetEnableTargetWidget`
  (params (bIsSelected :type Boolean))
  (bind _targetframe (`self.TargetFrame`))
  (bind (_returnvalue_roll _returnvalue_pitch) (`KismetMathLibrary.BreakRotator` (`SceneComponent.K2_GetComponentRotation` _targetframe)))
  (bind (_returnvalue_roll_2 _returnvalue_pitch_2 _returnvalue_yaw) (`KismetMathLibrary.BreakRotator` (`KismetMathLibrary.FindLookAtRotation` (`self.K2_GetActorLocation`) (`self.K2_GetActorLocation` (`GameplayStatics.GetPlayerCharacter` 0)))))
  (if bIsSelected
    (`KismetSystemLibrary.PrintString` (`KismetStringLibrary.Concat_StrStr` "update widget inside" (`KismetSystemLibrary.GetDisplayName` self)) false)
    (`/Game/UserInterface/Widgets/Combat/W_Target.ShowTarget` (`self.As W Target`))
    ;[1 1 1] Do it with a timer
    (`SceneComponent.K2_SetWorldRotation` _targetframe (`KismetMathLibrary.MakeRotator` _returnvalue_roll _returnvalue_pitch _returnvalue_yaw) false false)
    (bind _returnvalue (`KismetSystemLibrary.K2_SetTimer` null "UpdateWidgetRotation" 0.004167 true))
    (set `self.UpdateWidgetRotationTimer` _returnvalue)
    (else
      (`/Game/UserInterface/Widgets/Combat/W_Target.HideTarget` (`self.As W Target`))
      (`KismetSystemLibrary.K2_ClearAndInvalidateTimerHandle` (`self.UpdateWidgetRotationTimer`)))))

(event `self.ReceiveTick`
  (params (DeltaSeconds :type "Float (single-precision)"))
  (bind _parry (`self.Parry`))
  (bind (_returnvalue_roll _returnvalue_pitch) (`KismetMathLibrary.BreakRotator` (`SceneComponent.K2_GetComponentRotation` _parry)))
  (bind (_returnvalue_roll_2 _returnvalue_pitch_2 _returnvalue_yaw) (`KismetMathLibrary.BreakRotator` (`KismetMathLibrary.FindLookAtRotation` (`self.K2_GetActorLocation`) (`self.K2_GetActorLocation` (`GameplayStatics.GetPlayerCharacter` 0)))))
  (`SceneComponent.K2_SetWorldRotation` _parry (`KismetMathLibrary.MakeRotator` _returnvalue_roll _returnvalue_pitch _returnvalue_yaw) false false)
  (if (`self.Was Parried`)
    (`/Game/UserInterface/Widgets/Combat/W_ParryIcon.SetActive` (`self.As W Parry Icon`) false)))

(fn `TakeDamage`
  (set `self.Health` 0.0))

(fn `UpdateWidgetRotation`
  (bind _targetframe (`self.TargetFrame`))
  (bind (_returnvalue_roll _returnvalue_pitch) (`KismetMathLibrary.BreakRotator` (`SceneComponent.K2_GetComponentRotation` _targetframe)))
  (bind (_returnvalue_roll_2 _returnvalue_pitch_2 _returnvalue_yaw) (`KismetMathLibrary.BreakRotator` (`KismetMathLibrary.FindLookAtRotation` (`self.K2_GetActorLocation`) (`self.K2_GetActorLocation` (`GameplayStatics.GetPlayerCharacter` 0)))))
  (`SceneComponent.K2_SetWorldRotation` _targetframe (`KismetMathLibrary.MakeRotator` _returnvalue_roll _returnvalue_pitch _returnvalue_yaw) false false))

(fn `UserConstructionScript`)